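; HealthPot is a health potion item that the custom third-person character can pick up, carry, drop or consume.
; Overlap asks the character to pick it up, and Pickup attaches the Base component to the mesh's right-hand socket.
; Drop detaches DefaultSceneRoot and enables physics and collision on Base.
; PrimaryAction only prints a health message, clears the character's held item and destroys the actor, without changing any health value.
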(event OnComponentBeginOverlap(HealthPot)
  (params (OverlappedComponent :type Primitive%20Component%20Object%20Reference) (OtherActor :type Actor%20Object%20Reference) (OtherComp :type Primitive%20Component%20Object%20Reference) (OtherBodyIndex :type Integer) (bFromSweep :type Boolean) (SweepResult :type Hit%20Result%20Structure%20%28by%20ref%29))
  (bind _asbp_third_person_character_custome (Utilities|Casting|CastToBP_ThirdPersonCharacterCustome OtherActor))
  (Default|TrytoPickUP _asbp_third_person_character_custome self))

(event EventPickup
  (params (ParentMesh :type Skeletal%20Mesh%20Component%20Object%20Reference))
  (Transformation|AttachComponentToComponent (Variables|Default|GetBase) ParentMesh "hand_r" "KeepRelative" "KeepRelative" "KeepRelative" true))

(event EventDrop
  (Transformation|DetachFromComponent (Variables|Default|GetDefaultSceneRoot) "KeepRelative" "KeepRelative" "KeepRelative" true)
  (Physics|SetSimulatePhysics (Variables|Default|GetBase) true)
  (Collision|SetCollisionEnabled (Variables|Default|GetBase) "QueryAndPhysics"))

(event EventPrimaryAction
  (params (ref_ThirdPersonCharCustom :type BP%20Third%20Person%20Character%20Custome%20Object%20Reference))
  (Development|PrintString "+10 Health")
  (Variables|/Game/Blueprints/BP_ThirdPersonCharacterCustome.BP_ThirdPersonCharacterCustome_C|SetHeld%20Item ref_ThirdPersonCharCustom 0)
  (Actor|DestroyActor))

(fn ConstructionScript)