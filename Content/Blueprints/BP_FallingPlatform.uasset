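; BP_FallingPlatform is a platform that falls after the custom third-person character overlaps its trigger box, then returns to its starting place.
; Overlap starts a Ready-gated chain of delayed Active, Drop and Reset events that enables physics on the Cube to drop it.
; Reset disables physics and uses a Timeline to lerp the Cube from its landed transform back to the one saved at BeginPlay.
; Material color swaps and debug prints mark each state.
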(event OnComponentBeginOverlap(Box)
  (params (OverlappedComponent :type Primitive%20Component%20Object%20Reference) (OtherActor :type Actor%20Object%20Reference) (OtherComp :type Primitive%20Component%20Object%20Reference) (OtherBodyIndex :type Integer) (bFromSweep :type Boolean) (SweepResult :type Hit%20Result%20Structure%20%28by%20ref%29))
  (Utilities|Casting|CastToBP_ThirdPersonCharacterCustome OtherActor)
  (CallFunction|Active))

(event Custom|Active
  (if (Variables|Default|GetReady)
    (Development|PrintString "1 Beer left!")
    (Variables|Default|SetReady false)
    (Rendering|Material|SetMaterial (Variables|Default|GetCube) 0 "/Game/LevelPrototyping/Materials/MI_Solid_Yellow.MI_Solid_Yellow")
    (Utilities|FlowControl|Delay 2.0)
    (CallFunction|Drop)))

(event Custom|Drop
  (Development|PrintString "Fallin'")
  (Rendering|Material|SetMaterial (Variables|Default|GetCube) 0 "/Game/LevelPrototyping/Materials/MI_Solid_Red.MI_Solid_Red")
  (Physics|SetSimulatePhysics (Variables|Default|GetCube) true)
  (Utilities|FlowControl|Delay 3.0)
  (CallFunction|Reset))

(event Custom|Reset
  (Development|PrintString "Resetting")
  (Rendering|Material|SetMaterial (Variables|Default|GetCube) 0 "/Game/LevelPrototyping/Materials/MI_Solid_Blue.MI_Solid_Blue")
  (Variables|Default|SetResetTransform (Transformation|GetWorldTransform (Variables|Default|GetCube)))
  (Physics|SetSimulatePhysics (Variables|Default|GetCube) false)
  (bind _resettin (Timeline|Timeline PlayFromStart)
    (:Update
      (Transformation|SetWorldLocationAndRotation (Variables|Default|GetCube) (.location (Math|Transform|Lerp(Transform) (Variables|Default|GetResetTransform) (Variables|Default|GetStartingTransform) _resettin)) (.rotation (Math|Transform|Lerp(Transform) (Variables|Default|GetResetTransform) (Variables|Default|GetStartingTransform) _resettin)) false false))
    (:Finished
      (Variables|Default|SetReady true)
      (Rendering|Material|SetMaterial (Variables|Default|GetCube) 0 "/Game/LevelPrototyping/Materials/MI_Solid_Green.MI_Solid_Green"))))

(event EventBeginPlay
  (Variables|Default|SetStartingTransform (Transformation|GetWorldTransform (Variables|Default|GetCube))))

(event Collision|EventActorBeginOverlap
  (params (OtherActor :type Actor%20Object%20Reference)))

(event EventTick
  (params (DeltaSeconds :type Float%20%28single-precision%29)))

(fn ConstructionScript)