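; Key pickup actor that the player collects by walking into its box trigger.
; On overlap with BP_ThirdPersonCharacterCustome it increments the character's KeyCount and prints the new total.
; The cylinder mesh then turns red and the actor destroys itself after a short delay, with no guard against repeat overlaps during that wait.
; Debug prints also report its spawn and failed casts from other actors.
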(event OnComponentBeginOverlap(Box)
  (params (OverlappedComponent :type Primitive%20Component%20Object%20Reference) (OtherActor :type Actor%20Object%20Reference) (OtherComp :type Primitive%20Component%20Object%20Reference) (OtherBodyIndex :type Integer) (bFromSweep :type Boolean) (SweepResult :type Hit%20Result%20Structure%20%28by%20ref%29))
  (bind _asbp_third_person_character_custome (Utilities|Casting|CastToBP_ThirdPersonCharacterCustome OtherActor)
    (:then
      (Development|PrintString "A player ran into key" true true "(R=0.000000,G=0.660000,B=1.000000,A=1.000000)" 5.0)
      (Variables|/Game/Blueprints/BP_ThirdPersonCharacterCustome.BP_ThirdPersonCharacterCustome_C|SetKeyCount _asbp_third_person_character_custome (+ (Variables|/Game/Blueprints/BP_ThirdPersonCharacterCustome.BP_ThirdPersonCharacterCustome_C|GetKeyCount _asbp_third_person_character_custome) 1))
      (Development|PrintString (Utilities|String|Append "The Player has" (Utilities|String|ToString(Integer) (Variables|/Game/Blueprints/BP_ThirdPersonCharacterCustome.BP_ThirdPersonCharacterCustome_C|GetKeyCount _asbp_third_person_character_custome)) "keys"))
      (Rendering|Material|SetMaterial (Variables|Default|GetCylinder) 0 "/Game/LevelPrototyping/Materials/MI_Solid_Red.MI_Solid_Red")
      (Utilities|FlowControl|Delay 1.0)
      (Actor|DestroyActor))
    (:CastFailed
      (Development|PrintString "key get failed" true true "(R=1.000000,G=0.000000,B=0.035905,A=1.000000)"))))

(event EventBeginPlay
  (Development|PrintString "Key Exists"))

(event Collision|EventActorBeginOverlap
  (params (OtherActor :type Actor%20Object%20Reference)))

(event EventTick
  (params (DeltaSeconds :type Float%20%28single-precision%29)))

(fn ConstructionScript)