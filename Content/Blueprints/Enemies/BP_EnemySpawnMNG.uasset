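; Enemy spawn manager that places waves of BP_Enemy at every BP_Spawner in the level.
; On BeginPlay it gathers the spawners, spawns one enemy at each, hands each a reference to itself and counts them.
; EnemyCheck decrements the live count and, once none remain, respawns the wave after a short delay.
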(event Custom|SpawnEnemies
  (for _array_element (Variables|Default|GetSpawners)
    (bind _returnvalue (Game|SpawnActorfromClass "/Game/Blueprints/Enemies/BP_Enemy.BP_Enemy_C" (Math|Transform|MakeTransform (.location (Transformation|GetWorldTransform (Variables|/Game/Blueprints/Enemies/BP_Spawner.BP_Spawner_C|GetDefaultSceneRoot _array_element))) (.rotation (Transformation|GetWorldTransform (Variables|/Game/Blueprints/Enemies/BP_Spawner.BP_Spawner_C|GetDefaultSceneRoot _array_element))) "1.000000,1.000000,1.000000") "Undefined" "MultiplyWithRoot" 0 0))
    (Variables|/Game/Blueprints/Enemies/BP_Enemy.BP_Enemy_C|SetManager _returnvalue self)
    (Math|Integer|IncrementInt (Variables|Default|GetcurrEnemy))))

(event Custom|EnemyCheck
  (Math|Integer|DecrementInt (Variables|Default|GetcurrEnemy)
    (:%20%20
      (if (not (> (Variables|Default|GetcurrEnemy) 0))
        (Development|PrintString "respawning.." true true "(R=0.000000,G=0.660000,B=1.000000,A=1.000000)" 5.0)
        (Utilities|FlowControl|Delay 5.0)
        (CallFunction|SpawnEnemies)))))

(event EventBeginPlay
  (Development|PrintString "Enenmy Spawn Manager active")
  (bind _outactors (Actor|GetAllActorsOfClass "/Game/Blueprints/Enemies/BP_Spawner.BP_Spawner_C"))
  (Variables|Default|SetSpawners _outactors)
  (CallFunction|SpawnEnemies))

(fn ConstructionScript)